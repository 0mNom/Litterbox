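; VR climbing actor, named walk, that lets the player pull the MotionControllerPawnCourtney pawn around by gripping with motion controllers.
; Climb and LetGo track up to two gripping controllers, update the pawn's ClimbingHands count and reset the pivot point.
; While the pawn is climbing, Tick offsets it by the active controller's drift from the pivot, then pins that controller there.
; The second hand takes priority; releasing either hands control to the remaining one.
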(event EventBeginPlay)

(event Collision|EventActorBeginOverlap
  (params (OtherActor :type Actor%20Object%20Reference)))

(event EventTick
  (params (DeltaSeconds :type Float%20%28single-precision%29))
  (bind _firstmotioncontroller (Variables|Default|GetFirstMotionController))
  (bind _secondmotioncontroller (Variables|Default|GetSecondMotioncontroller))
  (bind _secondmotioncontroller_2 (Variables|Default|GetSecondMotioncontroller))
  (bind _returnvalue (Utilities|IsValid _secondmotioncontroller_2))
  (bind _returnvalue_2 (select _returnvalue _secondmotioncontroller _firstmotioncontroller))
  (if (Utilities|IsValid (Variables|Default|GetMotioncontrollerPawn))
    (if (and (Variables|/Game/Courtney/Blueprints/MotionControllerPawnCourtney.MotionControllerPawnCourtney_C|GetIsClimbing (Variables|Default|GetMotioncontrollerPawn)) (Utilities|IsValid (Variables|Default|GetFirstMotionController)))
      (Transformation|AddActorWorldOffset (Variables|Default|GetMotioncontrollerPawn) (- (Variables|Default|GetPivotPoint) (Transformation|GetWorldLocation _returnvalue_2)))
      (Transformation|SetWorldLocation _returnvalue_2 (Variables|Default|GetPivotPoint) false false))))

(event EventClimb
  (params (Motion%20Controller :type Scene%20Component%20Object%20Reference))
  ;[1 0 0.9375] Climbing
  (if (Utilities|IsValid (Variables|Default|GetFirstMotionController))
    (Variables|Default|SetSecondMotioncontroller Motion%20Controller)
    (else
      (Variables|Default|SetFirstMotionController Motion%20Controller)))
  (Variables|Default|SetPivotPoint (Transformation|GetWorldLocation (select (Utilities|IsValid (Variables|Default|GetSecondMotioncontroller)) (Variables|Default|GetSecondMotioncontroller) (Variables|Default|GetFirstMotionController))))
  (bind _asmotion_controller_pawn_courtney (Utilities|Casting|CastToMotionControllerPawnCourtney (Game|Player|GetPlayerPawn 0)))
  (bind _output_get (Variables|Default|SetMotioncontrollerPawn _asmotion_controller_pawn_courtney))
  (Math|Integer|IncrementInt (Variables|/Game/Courtney/Blueprints/MotionControllerPawnCourtney.MotionControllerPawnCourtney_C|GetClimbingHands _output_get)))

(event EventLetGo
  (params (Motion%20controller :type Scene%20Component%20Object%20Reference))
  ;[0.3359 0 1] Letting GO/Falling
  (if (Utilities|IsValid (Variables|Default|GetSecondMotioncontroller))
    (if (== Motion%20controller (Variables|Default|GetSecondMotioncontroller)) ; it was second hand that let o
      (Variables|Default|SetSecondMotioncontroller 0)
      (Variables|Default|SetPivotPoint (Transformation|GetWorldLocation (Variables|Default|GetFirstMotionController)))
      (else
        (Variables|Default|SetFirstMotionController (Variables|Default|GetSecondMotioncontroller))
        (Variables|Default|SetSecondMotioncontroller 0)
        (Variables|Default|SetPivotPoint (Transformation|GetWorldLocation (Variables|Default|GetFirstMotionController)))))
    (Math|Integer|DecrementInt (Variables|/Game/Courtney/Blueprints/MotionControllerPawnCourtney.MotionControllerPawnCourtney_C|GetClimbingHands (Variables|Default|GetMotioncontrollerPawn)) :!label _label)
    (elif (== Motion%20controller (Variables|Default|GetFirstMotionController)) ; No more hands holding
      (Variables|Default|SetFirstMotionController 0)
      (Variables|Default|SetSecondMotioncontroller 0)
      (Variables|Default|SetPivotPoint "0, 0, 0")
      (goto _label))))

(fn ConstructionScript)