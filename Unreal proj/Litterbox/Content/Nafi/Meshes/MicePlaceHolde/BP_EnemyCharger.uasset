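; Enemy charger that chases the first-person player and, on contact, sends them to a fixed location elsewhere in the world.
; PawnSensing spots the player and starts an AI MoveTo toward them.
; A hit teleports the player with a set rotation, plays a quiet Gregorian choir sound at a fixed point and moves the charger to its own preset position.
; A MoveComponentTo node is left unconnected and never runs.
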(event OnSeePawn(PawnSensing)
  (params (Pawn :type Pawn%20Object%20Reference))
  (bind _asfirst_person_character (Utilities|Casting|CastToFirstPersonCharacter Pawn))
  (AI|AIMoveTo self "0, 0, 0" _asfirst_person_character 5.0 false))

(event EventBeginPlay)

(event Collision|EventActorBeginOverlap
  (params (OtherActor :type Actor%20Object%20Reference)))

(event EventTick
  (params (DeltaSeconds :type Float%20%28single-precision%29)))

(event Collision|EventHit
  (params (MyComp :type Primitive%20Component%20Object%20Reference) (Other :type Actor%20Object%20Reference) (OtherComp :type Primitive%20Component%20Object%20Reference) (bSelfMoved :type Boolean) (HitLocation :type Vector :default "0, 0, 0") (HitNormal :type Vector :default "0, 0, 0") (NormalImpulse :type Vector :default "0, 0, 0") (Hit :type Hit%20Result%20Structure%20%28by%20ref%29))
  (Utilities|Casting|CastToFirstPersonCharacter Other)
  (Transformation|SetActorLocation (Game|GetPlayerCharacter 0) "9800.000000,-25930.000000,-46730.000000" false false)
  (Transformation|SetActorRotation (Game|GetPlayerCharacter 0) "0,90.000000, 0")
  (Audio|PlaySoundatLocation "/Game/Assets/looperman-l-0379853-0032783-alen9r-gregorian-choir-pad.looperman-l-0379853-0032783-alen9r-gregorian-choir-pad" "9260.000000,-32580.000000,-57660.000000" "0, 0, 0" 0.1 1.0 18.0 0 0 0)
  (Transformation|SetActorLocation "1000.000488,830.000000,-2313.897217" false false))

(fn ConstructionScript)