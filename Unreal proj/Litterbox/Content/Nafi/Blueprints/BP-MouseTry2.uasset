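; BP-MouseTry2 is an AI pawn, apparently a mouse, that wanders at random.
; Tick runs through a random delay of a few seconds, then sends it via AIMoveTo to a random reachable navmesh point around its current location.
; A Mov flag is set while moving and cleared on success or failure.
; PawnSensing's see event is empty, and logic for chasing, lifting, and teleporting the player with a sound is disconnected.
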(event OnSeePawn(PawnSensing)
  (params (Pawn :type Pawn%20Object%20Reference)))

(event EventBeginPlay)

(event Collision|EventActorBeginOverlap
  (params (OtherActor :type Actor%20Object%20Reference)))

(event EventTick
  (params (DeltaSeconds :type Float%20%28single-precision%29))
  (Utilities|FlowControl|Delay (Math|Random|RandomFloatinRange 1.0 3.0))
  (Variables|Default|SetMov true)
  (AI|AIMoveTo self (.RandomLocation (AI|Navigation|GetRandomReachablePointinRadius (Transformation|GetActorLocation) 2e+03 0 0)) 0 5.0 false
    (:OnSuccess
      _)
    (:OnFail
      _))
  (Variables|Default|SetMov false))

(event Collision|EventHit
  (params (MyComp :type Primitive%20Component%20Object%20Reference) (Other :type Actor%20Object%20Reference) (OtherComp :type Primitive%20Component%20Object%20Reference) (bSelfMoved :type Boolean) (HitLocation :type Vector :default "0, 0, 0") (HitNormal :type Vector :default "0, 0, 0") (NormalImpulse :type Vector :default "0, 0, 0") (Hit :type Hit%20Result%20Structure%20%28by%20ref%29)))

(fn ConstructionScript)