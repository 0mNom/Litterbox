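; LightAct_Blueprint holds light intensity and colour state and records when it is hit.
; BeginPlay initialises two intensity variables and sets the second colour to white.
; Each Hit event increments a click counter and raises a hit flag; no graph here applies these values to a light.
; A disconnected branch holds an unused dark blue colour setup, and the construction script is empty.
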(event EventBeginPlay
  (Utilities|FlowControl|Sequence
    (:then_0
      (Variables|Default|SetLightIntensity 1.5))
    (:then_1
      (Variables|Default|SetLightIntensity2 2.75)
      (Variables|Default|SetColour2 "(R=1.000000,G=1.000000,B=1.000000,A=1.000000)"))))

(event Collision|EventActorBeginOverlap
  (params (OtherActor :type Actor%20Object%20Reference)))

(event EventTick
  (params (DeltaSeconds :type Float%20%28single-precision%29)))

(event Collision|EventHit
  (params (MyComp :type Primitive%20Component%20Object%20Reference) (Other :type Actor%20Object%20Reference) (OtherComp :type Primitive%20Component%20Object%20Reference) (bSelfMoved :type Boolean) (HitLocation :type Vector :default "0, 0, 0") (HitNormal :type Vector :default "0, 0, 0") (NormalImpulse :type Vector :default "0, 0, 0") (Hit :type Hit%20Result%20Structure%20%28by%20ref%29))
  (Variables|Default|SetCountClick (+ (Variables|Default|GetCountClick) 1))
  (Variables|Default|SetIshit2 true))

(fn ConstructionScript)